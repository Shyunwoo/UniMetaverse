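; BP_MediaScreen is a media screen Blueprint that plays and pauses a media source through a MediaPlayer.
; StartMediaPlay resumes a paused player from where it stopped and otherwise opens the MediaSource, while PauseMediaPlay pauses a valid player.
; A WitchComputer macro routes execution to server, owning client or other client by authority and owner, though neither playback event uses it.
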(event Custom|StartMediaPlay
  ;[1 1 1] 미디어 플레이 일시정지면 멈춘곳에서 다시재생
  (if (Class|MediaPlayer|IsPaused (Variables|Default|GetMediaPlayer))
    (Media|MediaPlayer|Play (Variables|Default|GetMediaPlayer) :!class /Script/MediaAssets.MediaPlayer)
    (else
      (Media|MediaPlayer|OpenSource (Variables|Default|GetMediaPlayer) (Variables|Default|GetMedia%20Source)))))

(event Custom|PauseMediaPlay
  (bind _mediaplayer (Variables|Default|GetMediaPlayer))
  ;[1 1 1] 미디어 일시정지
  (Utilities|IsValid _mediaplayer
    (:Is%20Valid
      (Sequencer|Player|Pause _mediaplayer))))

(fn ConstructionScript)