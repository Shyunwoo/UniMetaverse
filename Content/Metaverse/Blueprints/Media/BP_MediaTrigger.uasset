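; BP_MediaTrigger is a trigger volume that controls playback on a linked MediaScreen as the player enters and leaves it.
; Box overlap events start media on entry and pause it on exit, only when the BP_DeajinCharacter is player 0's controlled pawn.
; A WitchComputer macro, not called in the event graph, branches into Server, MyClient or OtherClient by authority and owning controller.
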(event OnComponentBeginOverlap(Box)
  (params (OverlappedComponent :type Primitive%20Component%20Object%20Reference) (OtherActor :type Actor%20Object%20Reference) (OtherComp :type Primitive%20Component%20Object%20Reference) (OtherBodyIndex :type Integer) (bFromSweep :type Boolean) (SweepResult :type Hit%20Result%20Structure%20%28by%20ref%29))
  ;[1 1 1] 캐릭터가 오버랩되면 미디어 플레이 이벤트 호출
  (bind _asbp_deajin_character (Utilities|Casting|CastToBP_DeajinCharacter OtherActor))
  (if (== _asbp_deajin_character (Pawn|GetControlledPawn (Game|GetPlayerController 0)))
    (Default|StartMediaPlay (Variables|Default|GetMediaScreen))))

(event OnComponentEndOverlap(Box)
  (params (OverlappedComponent :type Primitive%20Component%20Object%20Reference) (OtherActor :type Actor%20Object%20Reference) (OtherComp :type Primitive%20Component%20Object%20Reference) (OtherBodyIndex :type Integer))
  ;[1 1 1] 캐릭터가 엔드 오버랩되면 미디어 일시정지 이벤트 호출
  (bind _asbp_deajin_character (Utilities|Casting|CastToBP_DeajinCharacter OtherActor))
  (if (== _asbp_deajin_character (Pawn|GetControlledPawn (Game|GetPlayerController 0)))
    (Default|PauseMediaPlay (Variables|Default|GetMediaScreen))))

(fn ConstructionScript)