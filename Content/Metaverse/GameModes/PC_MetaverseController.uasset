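; Player controller for the Metaverse world, handling each user's HUD, identity, chat and YouTube live stream.
; On BeginPlay, remote clients create the player widget, start audio and open any stream URL already set in GameState.
; Possession passes the GameInstance's saved name and mesh index to the server's PlayerState.
; Chat relays through the GameMode's controller list, Enter focuses its entry box, and new stream URLs go to GameState.
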(event Custom|ResClientPosses
  ;[1 1 1] 클라이언트 빙의 이벤트 수신
  (bind _asgi_metaverse_instance (Utilities|Casting|CastToGI_MetaverseInstance (Game|GetGameInstance)))
  (Utilities|IsValid _asgi_metaverse_instance
    (:Is%20Valid
      (CallFunction|ReqSetNewName (Variables|/Game/Metaverse/GameModes/GI_MetaverseInstance.GI_MetaverseInstance_C|GetSavedPlayerID _asgi_metaverse_instance) (Variables|/Game/Metaverse/GameModes/GI_MetaverseInstance.GI_MetaverseInstance_C|GetSavedPlayerInt _asgi_metaverse_instance)))))

(event Custom|ReqSetNewName
  (params (NewName :type String) (NewMesh :type Integer))
  ;[1 0 0] 서버 새로운 이름 적용
  (CallFunction|InitPlayerState NewName NewMesh))

(event Custom|GetChatMessage
  (params (TextToSend :type Text))
  ;[1 1 1] 전송받은 메세지를 처리하고 모든 사용자에게 메세지 전송
  (Variables|Default|SetSenderText TextToSend)
  (bind _asps_metaverse_player_state (Utilities|Casting|CastToPS_MetaversePlayerState (Variables|GetPlayerState)))
  (Variables|Default|SetChange%20Name (Utilities|Text|ToText(String) (Variables|/Game/Metaverse/GameModes/PS_MetaversePlayerState.PS_MetaversePlayerState_C|GetChangeName _asps_metaverse_player_state)))
  (bind _asgm_metaverse_gamemode (Utilities|Casting|CastToGM_MetaverseGamemode (Game|GetGameMode)))
  (for _array_element (Variables|/Game/Metaverse/GameModes/GM_MetaverseGamemode.GM_MetaverseGamemode_C|GetAlivePCs _asgm_metaverse_gamemode)
    (bind _aspc_metaverse_controller (Utilities|Casting|CastToPC_MetaverseController _array_element))
    (CallFunction|UpdateChat _aspc_metaverse_controller (Variables|Default|GetChange%20Name) (Variables|Default|GetSenderText))))

(event Custom|UpdateChat
  (params (Sender :type Text) (Text :type Text))
  ;[1 1 1] 채팅 출력 업데이트
  (Default|UpdateChatWindow (Variables|/Game/Metaverse/UI/WBP_PlayerWidget.WBP_PlayerWidget_C|GetWBP_ChatWindow (Variables|Default|GetRefPlayerWidget)) Sender Text))

(event Custom|ReqNewURL
  (params (NewURL :type String))
  (bind _returnvalue (Game|GetGameState))
  ;[1 0 0] 서버에서 URL 적용
  (Utilities|IsValid _returnvalue
    (:Is%20Valid
      (bind _asgs_metaverse_game_state (Utilities|Casting|CastToGS_MetaverseGameState _returnvalue))
      (Default|SetNewURL _asgs_metaverse_game_state NewURL))))

(event EventBeginPlay
  ;[1 1 1] 월드에 오면 게임모드 및 마우스 보기
  (Input|SetInputModeGameOnly self)
  (Variables|Default|SetbShowMouseCursor false)
  ;[1 1 1] 사용자가 접속하면 연결 후 위젯 띄우기
  (Networking|SwitchHasAuthority
    (:Remote
      (bind _returnvalue (UserInterface|CreateWidget "/Game/Metaverse/UI/WBP_PlayerWidget.WBP_PlayerWidget_C" self self))
      (bind _output_get (Variables|Default|SetRefPlayerWidget _returnvalue))
      (UserInterface|Viewport|AddtoViewport _output_get 0)
      (CallFunction|PlayAudio)
      ;[1 1 1] 이미 라이브가 재생중이면 라이브 플레이
      (bind _asgs_metaverse_game_state (Utilities|Casting|CastToGS_MetaverseGameState (Game|GetGameState)))
      (if (Variables|/Game/Metaverse/GameModes/GS_MetaverseGameState.GS_MetaverseGameState_C|GetSet%20URL _asgs_metaverse_game_state)
        (Variables|/Script/MediaAssets.StreamMediaSource|SetStreamUrl (Variables|Default|GetYoutubeLiveSource) (Variables|/Game/Metaverse/GameModes/GS_MetaverseGameState.GS_MetaverseGameState_C|GetStrYoutubeURL _asgs_metaverse_game_state))
        (Media|MediaPlayer|OpenSource (Variables|Default|GetYoutubeLivePlayer) (Variables|Default|GetYoutubeLiveSource))))))

(event EventPossess
  (params (PossessedPawn :type Pawn%20Object%20Reference))
  ;[1 0 0] 서버 빙의 이벤트
  (CallFunction|ResClientPosses))

(event Input|KeyboardEvents|Enter
  (params (Key :type Key%20Structure :default "None"))
  (bind _refplayerwidget (Variables|Default|GetRefPlayerWidget))
  (bind _wbp_chatwindow (Variables|/Game/Metaverse/UI/WBP_PlayerWidget.WBP_PlayerWidget_C|GetWBP_ChatWindow _refplayerwidget))
  (bind _entrychat (Variables|/Game/Metaverse/UI/WBP_ChatWindow.WBP_ChatWindow_C|GetEntryChat _wbp_chatwindow))
  (:Pressed
    ;[1 1 1] 엔터를 치면 채팅을 시작
    (Utilities|IsValid _refplayerwidget
      (:Is%20Valid
        (if (not (Class|Widget|HasKeyboardFocus _entrychat))
          (Input|SetInputModeGameandUI self _entrychat "DoNotLock" true))))))

(fn ConstructionScript)

(fn InitPlayerState
  (params (Name :type String) (IntMesh :type Integer))
  ;[1 1 1] 플레이어 스테이트 초기화
  (bind _asps_metaverse_player_state (Utilities|Casting|CastToPS_MetaversePlayerState (Variables|GetPlayerState))
    (:then
      (Utilities|IsValid _asps_metaverse_player_state
        (:Is%20Valid
          (Default|SetName _asps_metaverse_player_state Name)
          (Default|SetCharMeshInt _asps_metaverse_player_state IntMesh))))
    (:CastFailed
      (Utilities|Time|SetTimerbyFunctionName 0 "InitPlayerState" 0.01))))

(fn PauseAudio
  (Audio|Components|Audio|Stop (Variables|Default|GetAudio)))

(fn PlayAudio
  (Audio|Components|Audio|Play (Variables|Default|GetAudio) 0.0))