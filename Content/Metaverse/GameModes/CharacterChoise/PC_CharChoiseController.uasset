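; Player controller for the character selection screen of the metaverse game.
; On BeginPlay it sets the view to the first actor tagged MainCamera, then creates and displays the character choice widget with UI-only input and a visible cursor.
; The widget only appears if that tagged camera is found.
; An Escape key binding quits the game.
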(event EventBeginPlay
  (bind _outactors (Actor|GetAllActorswithTag "MainCamera"))
  (if (> (Utilities|Array|Length _outactors) 0)
    (bind _ascamera_actor (Utilities|Casting|CastToCameraActor (Utilities|Array|Get(acopy) _outactors)))
    (Game|Player|SetViewTargetwithBlend _ascamera_actor 0.0 "VTBlend_Linear" 0.0 false)
    ;[1 1 1] 캐릭터선택 위젯 생성
    (bind _returnvalue (UserInterface|CreateWidget "/Game/Metaverse/GameModes/CharacterChoise/WBP_CharChoiseWidget.WBP_CharChoiseWidget_C" self))
    (Utilities|IsValid _returnvalue
      (:Is%20Valid
        (bind _output_get (Variables|Default|SetRefCharChoiseWidget _returnvalue))
        (UserInterface|Viewport|AddtoViewport _output_get 0)
        (Input|SetInputModeUIOnly self 0 "DoNotLock")
        (Variables|Default|SetbShowMouseCursor true)))))

(event Input|KeyboardEvents|Escape
  (params (Key :type Key%20Structure :default "None"))
  (:Pressed
    (Game|QuitGame 0 "Quit" false)))

(fn ConstructionScript)