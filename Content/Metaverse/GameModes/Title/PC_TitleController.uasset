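; Player controller for the title screen that shows the title menu and handles its basic key input.
; On BeginPlay it creates the title widget, stores it, adds it to the viewport, and switches to game-and-UI input focused on it with the cursor visible.
; Enter opens the character choice level and Escape quits the game.
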(event EventBeginPlay
  ;[1 1 1] 타이틀화면 위젯생성
  (bind _returnvalue (UserInterface|CreateWidget "/Game/Metaverse/GameModes/Title/WBP_TitleWidget.WBP_TitleWidget_C" self))
  (Utilities|IsValid _returnvalue
    (:Is%20Valid
      (bind _output_get (Variables|Default|SetRef_TitleWidget _returnvalue))
      (UserInterface|Viewport|AddtoViewport _output_get 0)
      (Input|SetInputModeGameandUI self _output_get "DoNotLock" true)
      (Variables|Default|SetbShowMouseCursor true))))

(event Input|KeyboardEvents|Enter
  (params (Key :type Key%20Structure :default "None"))
  (:Pressed
    (Game|OpenLevel(byName) "CharacterChoiseLevel")))

(event Input|KeyboardEvents|Escape
  (params (Key :type Key%20Structure :default "None"))
  (:Pressed
    (Game|QuitGame 0 "Quit" false)))

(fn ConstructionScript)