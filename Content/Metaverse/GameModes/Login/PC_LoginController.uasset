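; Player controller for the Metaverse login game mode that shows the login screen and hands the player off to a server.
; On BeginPlay it creates the login widget, adds it to the viewport and switches to UI-only input with a visible cursor.
; JoinServer opens JoinLoadingLevel, passing the server IP as a NextMap option, and an Escape key binding quits the game.
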(event Custom|JoinServer
  (params (ServerIP :type String))
  ;[1 1 1] 서버의 아이피 주소로 이동
  (Game|OpenLevel(byName) "JoinLoadingLevel" true (Utilities|String|Append "NextMap=" ServerIP)))

(event EventBeginPlay
  ;[1 1 1] 로그인화면 위젯생성
  (bind _returnvalue (UserInterface|CreateWidget "/Game/Metaverse/GameModes/Login/WBP_LoginWidget.WBP_LoginWidget_C" self))
  (Utilities|IsValid _returnvalue
    (:Is%20Valid
      (bind _output_get (Variables|Default|SetRefLoginWidget _returnvalue))
      (UserInterface|Viewport|AddtoViewport _output_get 0)
      (Input|SetInputModeUIOnly self 0 "DoNotLock")
      (Variables|Default|SetbShowMouseCursor true))))

(event Input|KeyboardEvents|Escape
  (params (Key :type Key%20Structure :default "None"))
  (:Pressed
    (Game|QuitGame 0 "Quit" false)))

(fn ConstructionScript)